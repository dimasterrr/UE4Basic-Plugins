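; Level portal actor whose appearance shows whether the portal is enabled or disabled.
; The construction script calls UpdateVisual, which reads IsPortalEnabled to tint the light green or red and swap the static mesh's first material slot between two materials.
; The file contains only this visual logic, with no travel or overlap handling.
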(fn `Update Visual`
  (`|ExecutionSequence`
    (:`then_0`
      (`LightComponent.SetLightColor` (`self.Light`) (`KismetMathLibrary.SelectColor` (struct :`G` 1.0 :`B` 0.0852 :`A` 1.0) (struct :`R` 1.0 :`B` 0.079394 :`A` 1.0) (`self.IsPortalEnabled`)) true))
    (:`then_1`
      (`PrimitiveComponent.SetMaterial` (`self.StaticMesh`) 0 (select `bool` (`self.IsPortalEnabled`) :`false` "/Game/Assets/Meshes/Arc/Material1.Material1" :`true` "/Game/Assets/Meshes/Arc/Material.Material" :!type "MaterialInterface Object Reference")))))

(fn `UserConstructionScript`
  (`self.Update Visual`))